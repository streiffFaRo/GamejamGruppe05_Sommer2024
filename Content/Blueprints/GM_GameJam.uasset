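; Game mode for a game jam project that restores audio settings at startup and handles player respawning.
; On BeginPlay it loads or creates the SG_Audio save, applies master, music and SFX volumes as sound mix class overrides, then saves it.
; RespawnPlayer destroys the current character, spawns a new C_Player at LastCheckpoint and possesses it.
; The ending manager lookup has no effect, and the intro widget logic is disconnected.
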(event `self.ReceiveBeginPlay`
  (bind _savegameaudioref (`self.SaveGameAudioRef`))
  ;[1 1 1] Setup Audio
  (`|ExecutionSequence`
    (:`then_0`
      (bind _returnvalue (`GameplayStatics.DoesSaveGameExist` "SG_Audio"))
      (if _returnvalue
        (bind _returnvalue_2 (`GameplayStatics.LoadGameFromSlot` "SG_Audio"))
        (bind _assg_audio (cast `/Game/Audio/Sounds/Settings/SG_Audio` _returnvalue_2))
        (set `self.SaveGameAudioRef` _assg_audio)
        (else
          (bind _returnvalue_3 (`GameplayStatics.CreateSaveGameObject` "/Game/Audio/Sounds/Settings/SG_Audio.SG_Audio_C"))
          (set `self.SaveGameAudioRef` _returnvalue_3)))
      (`|ExecutionSequence`
        (:`then_0`
          (`GameplayStatics.SetSoundMixClassOverride` "/Game/Audio/Sounds/Settings/SCM_Default.SCM_Default" "/Game/Audio/Sounds/Settings/SC_Master.SC_Master" (`/Game/Audio/Sounds/Settings/SG_Audio.MasterValue` _savegameaudioref) 1.0 0.0)
          (`GameplayStatics.PushSoundMixModifier` "/Game/Audio/Sounds/Settings/SCM_Default.SCM_Default"))
        (:`then_1`
          (`GameplayStatics.SetSoundMixClassOverride` "/Game/Audio/Sounds/Settings/SCM_Default.SCM_Default" "/Game/Audio/Sounds/Settings/SC_Music.SC_Music" (`/Game/Audio/Sounds/Settings/SG_Audio.MusicValue` _savegameaudioref) 1.0 0.0)
          (`GameplayStatics.PushSoundMixModifier` "/Game/Audio/Sounds/Settings/SCM_Default.SCM_Default"))
        (:`then_2`
          (`GameplayStatics.SetSoundMixClassOverride` "/Game/Audio/Sounds/Settings/SCM_Default.SCM_Default" "/Game/Audio/Sounds/Settings/SC_Sounds.SC_Sounds" (`/Game/Audio/Sounds/Settings/SG_Audio.SFXValue` _savegameaudioref) 1.0 0.0)
          (`GameplayStatics.PushSoundMixModifier` "/Game/Audio/Sounds/Settings/SCM_Default.SCM_Default")))
      (`GameplayStatics.SaveGameToSlot` (`self.SaveGameAudioRef`) "SG_Audio"))
    (:`then_1`
      (bind _returnvalue_4 (`GameplayStatics.GetActorOfClass` "/Game/Blueprints/A_EndingManager.A_EndingManager_C"))
      (`/Engine/EditorBlueprintResources/StandardMacros.IsValid` _returnvalue_4))))

(event `Respawn Player`
  (bind (_returnvalue_location _returnvalue_rotation) (`KismetMathLibrary.BreakTransform` (`SceneComponent.K2_GetComponentToWorld` (`/Game/Blueprints/A_Checkpoint.POS` (`self.LastCheckpoint`)))))
  ;[1 1 1] Respawn Player
  (`self.K2_DestroyActor` (`GameplayStatics.GetPlayerCharacter` 0))
  (bind _returnvalue (`|SpawnActorFromClass` "/Game/Player/C_Player.C_Player_C" (`KismetMathLibrary.MakeTransform` _returnvalue_location _returnvalue_rotation) "AlwaysSpawn" "MultiplyWithRoot" null null))
  (`Controller.Possess` (`GameplayStatics.GetPlayerController` 0) _returnvalue))

(fn `UserConstructionScript`)